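; Pushable block that slides along Y when pushed and drops when it loses the ground beneath it.
; Push starts a looping timer that eases the block 50 units along +Y with FInterpTo, spawning dust particles.
; A timed downward trace detects missing ground, then cancels the push, disables movement and stops checking.
; The block then descends at FallSpeed until a short trace at Grounded hits a surface.
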(event Custom|Checkground
  (bind _stillonground (Variables|Default|GetStillOnGround))
  (bind _returnvalue (Transformation|GetWorldLocation _stillonground))
  (bind _returnvalue_2 (Collision|LineTraceByChannel _returnvalue (+ _returnvalue "0,0.000000,-200.000000") "TraceTypeQuery1" false 0 "ForOneFrame"))
  (if (not _returnvalue_2)
    (CallFunction|Stop)
    (CallFunction|Fall)
    (Utilities|Time|ClearandInvalidateTimerbyHandle (stale EventBeginPlay _returnvalue))))

(event Custom|Stop
  (Utilities|Time|ClearandInvalidateTimerbyHandle (Variables|Default|GetMoveTimerHandle)))

(event Custom|Fall
  ;[1 1 1] Fall block
  (bind _returnvalue (Utilities|Time|SetTimerbyEvent (delegate Custom|FallTimer) 0.016667 true))
  (Variables|Default|SetFallTimerHandle _returnvalue)
  (Utilities|Time|ClearandInvalidateTimerbyHandle (Variables|Default|GetMoveTimerHandle))
  (Variables|Default|SetCanMove false))

(event Custom|FallTimer
  (bind _grounded (Variables|Default|GetGrounded))
  (bind _returnvalue (Transformation|GetWorldLocation _grounded))
  ;[1 1 1] Fall block
  (Transformation|AddActorWorldOffset (Math|Vector|MakeVector 0.0 0.0 (* (Variables|Default|GetFallSpeed) -0.016667)))
  (bind _returnvalue_2 (Collision|LineTraceByChannel _returnvalue (+ _returnvalue "0, 0,-10.000000") "TraceTypeQuery1" false 0 "None"))
  (if _returnvalue_2
    (Utilities|Time|ClearandInvalidateTimerbyHandle (Variables|Default|GetFallTimerHandle))))

(event Custom|MoveTimer
  (bind _returnvalue (Transformation|GetActorLocation))
  (bind (_x _y _z) (Math|Vector|BreakVector _returnvalue))
  (if (Variables|Default|GetCanMove)
    (Transformation|SetActorLocation (Math|Vector|MakeVector _x (Math|Interpolation|FInterpTo _y (.Y (Math|Vector|BreakVector (Variables|Default|GetStartLocation))) 0.016667 2.0) _z) false false)
    (Niagara|SpawnSystematLocation "/Game/Life/Particule/NS_Dust.NS_Dust" (Transformation|GetWorldLocation (Variables|Default|GetParticle)))
    (if (Math|Vector|Equal(Vector) (Transformation|GetActorLocation) (Variables|Default|GetStartLocation) 1.0)
      (Utilities|Time|ClearandInvalidateTimerbyHandle (Variables|Default|GetMoveTimerHandle)))))

(event EventBeginPlay
  (bind _returnvalue (Utilities|Time|SetTimerbyEvent (delegate Custom|Checkground) 0.008333 true)))

(event EventPush
  (bind _returnvalue (Transformation|GetActorLocation))
  (bind (_x _y _z) (Math|Vector|BreakVector _returnvalue))
  (Variables|Default|SetStartLocation (Math|Vector|MakeVector _x (+ _y 5e+01) _z))
  (bind _returnvalue_2 (Utilities|Time|SetTimerbyEvent (delegate Custom|MoveTimer) 0.016667 true))
  (Variables|Default|SetMoveTimerHandle _returnvalue_2))

(fn ConstructionScript)