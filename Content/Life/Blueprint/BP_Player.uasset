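; Player character for a life-themed game, where a one-second Aging countdown cues a late-life sound, then ends in the credits.
; Movement follows control yaw with looping footsteps, and is blocked after the end or while fallen.
; Fall fills GetUpValue, which GetUp presses drain, with quicker presses draining more via a timer-driven Lerp.
; Work line-traces along world +Y to push BP_Work, and Escape toggles the pause menu.
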(event Custom|Fall
  (Variables|Default|SetGetUpValue 1e+02)
  (bind _returnvalue (Utilities|Time|SetTimerbyEvent (delegate Custom|TimerGetUp) 0.008333 true))
  (Variables|Default|SetTimerHandleGetUp _returnvalue))

(event Custom|TimerGetUp
  (if (>= (Variables|Default|GetValue) 2.0)
    (CallFunction|FGetUp)
    (else
      (Variables|Default|SetValue (+ (Variables|Default|GetValue) 0.008333)))))

(event Custom|F_GetUp
  (Variables|Default|SetGetUpValue (- (Variables|Default|GetGetUpValue) (Math|Float|Lerp 1e+01 0.1 (Math|Float|NormalizetoRange (Variables|Default|GetValue) 0.0001 2.0))))
  (Variables|Default|SetValue 0.0)
  (if (<= (Variables|Default|GetGetUpValue) 0.0)
    (Variables|Default|SetGetUpValue 0.0)
    (Utilities|Time|ClearandInvalidateTimerbyHandle (Variables|Default|GetTimerHandleGetUp))))

(event Custom|Aging
  (Variables|Default|SetTime (- (Variables|Default|GetTime) 1))
  (if (<= (Variables|Default|GetTime) 0)
    (Utilities|FlowControl|DoOnce false
      (:Completed
        (CallFunction|FEnd)))
    (elif (<= (Variables|Default|GetTime) 250)
      (Utilities|FlowControl|DoOnce false
        (:Completed
          (Audio|PlaySound2D "/Game/Life/Musique/message-to-bears-you-are-a-memory.message-to-bears-you-are-a-memory" 1.0 1.0 0.0 0 0))))))

(event EventBeginPlay
  (bind _returnvalue (UserInterface|CreateWidget "/Game/Life/Widget/WPB_Interface.WPB_Interface_C"))
  (UserInterface|Viewport|AddtoViewport _returnvalue 0)
  (Utilities|Time|SetTimerbyEvent (delegate Custom|Aging) 1.0 true))

(event Input|ActionEvents|InputActionGetUp
  (params (Key :type Key%20Structure :default "None"))
  (:Pressed
    (if (not (<= (Variables|Default|GetGetUpValue) 0.0))
      (CallFunction|FGetUp))))

(event Input|ActionEvents|InputActionWork
  (params (Key :type Key%20Structure :default "None"))
  (bind _returnvalue (Transformation|GetActorLocation))
  (:Pressed
    (if (Variables|Default|GetCondition)
      (Variables|Default|SetCondition false)
      (bind _outhit (Collision|LineTraceByChannel _returnvalue (+ _returnvalue "0,50.000000, 0") "TraceTypeQuery1" false 0 "None"))
      (bind _asbp_work (Utilities|Casting|CastToBP_Work (.HitActor (Collision|BreakHitResult _outhit)))
        (:then
          (Default|Push _asbp_work)
          (Utilities|FlowControl|Delay 1.0)
          (Variables|Default|SetCondition true))
        (:CastFailed
          (Variables|Default|SetCondition true))))))

(event Input|AxisEvents|InputAxisMove
  (params (AxisValue :type Float%20%28single-precision%29))
  (if (not (Variables|Default|GetIsEnd?))
    (if (not (> (Variables|Default|GetGetUpValue) 0.0))
      (Pawn|Input|AddMovementInput (Math|Vector|GetForwardVector (Math|Rotator|MakeRotator 0.0 0.0 (.Yaw (Math|Rotator|BreakRotator (Pawn|GetControlRotation :!class /Script/Engine.Pawn))))) AxisValue false)
      (if (> AxisValue 0.0)
        (Utilities|FlowControl|DoOnce false :!label _label
          (:Completed
            (Audio|PlaySound2D "/Game/Life/Sound/Player/SC_Footstep.SC_Footstep" 1.0 1.0 0.0 0 0)
            (Utilities|FlowControl|Delay (Math|Random|RandomFloatinRange 0.7 0.75))
            (goto _label Reset)))
        (else
          (goto _label Reset))))))

(event Input|KeyboardEvents|Escape
  (params (Key :type Key%20Structure :default "None"))
  (:Pressed
    (CallFunction|FPause)))

(fn ConstructionScript)

(fn FPause
  (bind _returnvalue (Game|GetPlayerController 0))
  (bind _returnvalue_2 (Game|GetPlayerController 0))
  (if (Game|IsGamePaused)
    (Game|SetGamePaused false)
    (Widget|RemovefromParent (Variables|Default|GetPauseRef))
    (Input|SetInputModeGameOnly _returnvalue)
    (Variables|/Script/Engine.PlayerController|SetbShowMouseCursor _returnvalue false)
    (return)
    (else
      (Game|SetGamePaused true)
      (bind _returnvalue_3 (UserInterface|CreateWidget "/Game/Life/Widget/WBP_Pause.WBP_Pause_C"))
      (bind _output_get (Variables|Default|SetPauseRef _returnvalue_3))
      (UserInterface|Viewport|AddtoViewport _output_get 0)
      (Input|SetInputModeGameandUI _returnvalue_2 (Variables|Default|GetPauseRef) "DoNotLock" true)
      (Variables|/Script/Engine.PlayerController|SetbShowMouseCursor _returnvalue_2 true)
      (return))))

(fn FEnd
  (bind _returnvalue (Game|GetPlayerController 0))
  (Variables|Default|SetIsEnd? true)
  (bind _returnvalue_2 (UserInterface|CreateWidget "/Game/Life/Widget/WBP_Credit.WBP_Credit_C"))
  (Default|PlayIntro _returnvalue_2)
  (UserInterface|Viewport|AddtoViewport _returnvalue_2 0)
  (Variables|/Script/Engine.PlayerController|SetbShowMouseCursor _returnvalue true)
  (Input|SetInputModeUIOnly _returnvalue _returnvalue_2 "DoNotLock"))