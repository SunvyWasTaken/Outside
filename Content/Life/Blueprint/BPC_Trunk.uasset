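; BPC_Trunk is a pushable tree trunk that wobbles when pushed and falls once its Life runs out.
; Each Push subtracts a random amount from Life and restarts the T_AlmostFall timeline.
; The timeline rotates the Scene component toward 90 degrees in world space, using the Fall track at zero Life or below and the Presque (almost-fall) track otherwise.
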(event EventPush
  (Variables|Default|SetLife (- (Variables|Default|GetLife) (Math|Random|RandomFloatinRange 1e+01 25.0)))
  (bind (_direction _presque _fall) (Timeline|T_AlmostFall PlayFromStart)
    (:Update
      (Transformation|SetWorldRotation (Variables|Default|GetScene) (Math|Rotator|Lerp(Rotator) "0, 0, 0" "0, 0,90.000000" (Math|Float|SelectFloat _fall _presque (<= (Variables|Default|GetLife) 0.0)) true) false false))))

(fn ConstructionScript
  (|CallParentFunction))